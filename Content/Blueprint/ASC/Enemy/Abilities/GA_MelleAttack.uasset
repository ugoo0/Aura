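; Enemy melee attack gameplay ability that plays a random tagged montage from the avatar's CombatInterface while facing its combat target.
; The montage's gameplay event triggers a radius query at the tagged combat socket, damaging every live non-friendly player found.
; Any hit fires the MelleAttack gameplay cue, and the ability ends after the event or montage finish.
; A debug sphere draws at a fixed size, independent of AttackRadius.
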(event Ability|EventActivateAbility
  (bind _output_get (Variables|Default|SetAvatarActor (.AvatarActor (Utilities|Struct|BreakGameplayAbilityActorInfo (Ability|GetActorInfo)))))
  (bind _ascombat_interface (Utilities|Casting|CastToCombatInterface _output_get))
  (if (> (Utilities|Array|Length (Class|CombatInterface|GetTagstoMontage _ascombat_interface)) 0)
    (Variables|Default|SetTagToMontage (Utilities|Array|Get(acopy) (Class|CombatInterface|GetTagstoMontage _ascombat_interface) (Math|Random|RandomIntegerinRange 0 (- (Utilities|Array|Length (Class|CombatInterface|GetTagstoMontage _ascombat_interface)) 1))))
    (bind _returnvalue (Class|CombatInterface|GetCombatTarget _ascombat_interface))
    (Class|CombatInterface|FacingtoTarget _ascombat_interface (Transformation|GetActorLocation _returnvalue))
    (|PlayMontageandWaitProxy "None" (.Montage (Utilities|Struct|BreakTagsToMontage (Variables|Default|GetTagToMontage))) 1.0 "None" true 1.0 0.0
      (:then
        (Ability|Tasks|WaitGameplayEvent (.MontageGameplayTag (Utilities|Struct|BreakTagsToMontage (Variables|Default|GetTagToMontage))) 0
          (:EventReceived
            (Rendering|Debug|DrawDebugSphere (Class|CombatInterface|GetCombatSocketLocation _ascombat_interface (.SocketGameplayTag (Utilities|Struct|BreakTagsToMontage (Variables|Default|GetTagToMontage)))) 45.0 12 "(R=1.000000,G=0.078125,B=0.078125,A=1.000000)" 1.0)
            (bind _outoverlayactors (Class|AuraAbilitySystemLibrary|GetLivePlayerswithRadius (Variables|Default|GetAvatarActor) (Utilities|Array|MakeArray (Variables|Default|GetAvatarActor)) (Class|CombatInterface|GetCombatSocketLocation _ascombat_interface (.SocketGameplayTag (Utilities|Struct|BreakTagsToMontage (Variables|Default|GetTagToMontage)))) (Variables|Default|GetAttackRadius)))
            (Variables|Default|SetIsHit false)
            (for _array_element _outoverlayactors
              (bind _returnvalue_2 (Class|AuraAbilitySystemLibrary|IsFriend (Variables|Default|GetAvatarActor) _array_element))
              (if (not _returnvalue_2)
                (Class|AuraAbilitySystemLibrary|ApplyDamageEffectforDamageEffectParms 0 (Class|AuraDamageGameplayAbility|GetDamageEffectParamsforTarget _array_element))
                (Variables|Default|SetIsHit true)))
            (if (Variables|Default|GetIsHit)
              (bind _returnvalue_3 (Class|CombatInterface|GetCombatTarget(Message) (Variables|Default|GetAvatarActor)))
              (Class|GameplayAbility|ExecuteGameplayCuewithParams "(TagName=\"GameplayCue.MelleAttack\")" (Ability|GameplayCue|MakeGameplayCueParameters :AggregatedTargetTags (GameplayTags|MakeGameplayTagContainerfromTag (.MontageGameplayTag (Utilities|Struct|BreakTagsToMontage (Variables|Default|GetTagToMontage)))) :Location (Class|CombatInterface|GetCombatSocketLocation _ascombat_interface (.SocketGameplayTag (Utilities|Struct|BreakTagsToMontage (Variables|Default|GetTagToMontage)))) :EffectCauser (Variables|Default|GetAvatarActor) :SourceObject _returnvalue_3)))
            (Ability|EndAbility))))
      (:OnCompleted
        (Ability|EndAbility :!label _label))
      (:OnBlendOut
        (goto _label))
      (:OnInterrupted
        (goto _label))
      (:OnCancelled
        (goto _label)))
    (else
      (Ability|EndAbility))))

(event Ability|EventOnEndAbility
  (params (bWasCancelled :type Boolean)))