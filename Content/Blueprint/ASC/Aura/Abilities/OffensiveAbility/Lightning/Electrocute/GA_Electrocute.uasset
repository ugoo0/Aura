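; Gameplay ability for Electrocute, a channeled lightning beam aimed under the mouse that chains from an enemy to additional targets.
; A montage event spawns ShockLoop cues and starts a looping timer that pays cost and applies damage each tick.
; Input release, unaffordable cost or main-target death ends it, with the server delaying early releases until the minimum spell time.
; Cleanup removes cues, applies damage-effect params to surviving enemies server-side and commits cooldown.
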(event Custom|UpdateApplyDamage
  (CallFunction|CostandApplyDamage))

(event Ability|EventActivateAbility
  (if (Utilities|DoesObjectImplementInterface (Ability|GetAvatarActorfromActorInfo) "/Script/Aura.CombatInterface")
    (bind _datahandle (|TargetDataUnderMouse)
      (:ValidData
        (Class|AuraBeamSpell|StoreMouseDataInfo (Ability|TargetData|GetHitResultfromTargetData _datahandle))
        (Class|AuraBeamSpell|StoreOwnerVariables)
        (Utilities|FlowControl|Sequence
          (:then_0
            (Class|CombatInterface|FacingtoTarget(Message) (Ability|GetAvatarActorfromActorInfo) (Variables|Default|GetMouseHitLocation))
            (Variables|/Script/Engine.PlayerController|SetbShowMouseCursor (Variables|Default|GetOwnerPlayerController) false)
            (GameplayCue|AddGameplayCue :GameplayCueTag "(TagName=\"GameplayCue.ShockBurst\")")
            (|PlayMontageandWaitProxy "None" (Variables|Default|GetMontage_Electrocute) 1.0 "None" true 1.0 0.0
              (:then
                (Ability|Tasks|WaitGameplayEvent "(TagName=\"Event.Montage.Electrocute\")" 0 true
                  (:EventReceived
                    (Class|CombatInterface|SetinShockLoop(Message) (Ability|GetAvatarActorfromActorInfo) true)
                    (CallFunction|SpawnBeam)
                    (CallFunction|CostandApplyDamage)
                    (bind _returnvalue (Utilities|Time|SetTimerbyEvent (delegate Custom|UpdateApplyDamage) (Variables|Default|GetFrequencyApplyDamage) true))
                    (Variables|Default|SetTimerHandle _returnvalue))))))
          (:then_1
            (bind _timeheld (Ability|Tasks|WaitInputRelease false)
              (:then
                (bind _output_get (Variables|Default|SetHeldTime _timeheld)))
              (:OnRelease
                (if (> _output_get (Variables|Default|GetSpellTime))
                  (CallFunction|PreparetoEndAbility)
                  (Ability|EndAbility)
                  (else
                    (Ability|HasAuthority
                      (:True
                        (Utilities|FlowControl|Delay (- (Variables|Default|GetSpellTime) (Variables|Default|GetHeldTime)))
                        (CallFunction|PreparetoEndAbility)
                        (Ability|EndAbility))
                      (:False
                        (CallFunction|PreparetoEndAbility)))))))))))
    (else
      (Ability|EndAbility))))

(event EventMouseHitActorDead
  (params (HitActor :type Actor%20Object%20Reference))
  (Ability|HasAuthority
    (:True
      (CallFunction|PreparetoEndAbility)
      (Ability|EndAbility))
    (:False
      (CallFunction|PreparetoEndAbility))))

(event EventAdditionalActorDead
  (params (AdditionalActor :type Actor%20Object%20Reference))
  (bind _actortogcparam (Variables|Default|GetActorToGCParam))
  (bind (_value _returnvalue) (Utilities|Map|Find _actortogcparam AdditionalActor))
  (if _returnvalue
    (GameplayCue|RemoveGameplayCueOnActor(Looping) AdditionalActor "(TagName=\"GameplayCue.ShockLoop\")" _value)
    (Utilities|Array|RemoveItem (Variables|Default|GetOutAdditionalTargets) AdditionalActor)))

(event Ability|EventOnEndAbility
  (params (bWasCancelled :type Boolean))
  (Variables|/Script/Engine.PlayerController|SetbShowMouseCursor (Variables|Default|GetOwnerPlayerController) true))

(fn SpawnBeam
  (bind _mousehitactor (Variables|Default|GetMouseHitActor))
  (bind _returnvalue (Utilities|DoesObjectImplementInterface _mousehitactor "/Script/Aura.CombatInterface"))
  (Class|AuraBeamSpell|TraceFirstTarget (Variables|Default|GetMouseHitLocation))
  (bind _returnvalue_2 (Class|CombatInterface|GetWeapon(Message) (Ability|GetAvatarActorfromActorInfo)))
  (Variables|Default|SetFirstTargetCueParam (Ability|GameplayCue|MakeGameplayCueParameters :Location (Variables|Default|GetMouseHitLocation) :SourceObject (Variables|Default|GetMouseHitActor) :TargetAttachComponent _returnvalue_2))
  (Variables|Default|SetIsFirstHitIsEnemy _returnvalue)
  (if _returnvalue
    (Variables|Default|SetCueTarget (Variables|Default|GetMouseHitActor))
    (bind _outadditionaltargets (Class|AuraBeamSpell|StoreAdditionalTarget))
    (Variables|Default|SetOutAdditionalTargets _outadditionaltargets)
    (else
      (Variables|Default|SetCueTarget (Ability|GetAvatarActorfromActorInfo))))
  (GameplayCue|AddGameplayCueOnActor(Looping) (Variables|Default|GetCueTarget) "(TagName=\"GameplayCue.ShockLoop\")" (Variables|Default|GetFirstTargetCueParam))
  (Class|CombatInterface|SetIsBeingShock(Message) (Variables|Default|GetCueTarget) true)
  (if (Variables|Default|GetIsFirstHitIsEnemy)
    (CallFunction|SpreadBeam)))

(fn PreparetoEndAbility
  (if (Utilities|Time|IsValidTimerHandle (Variables|Default|GetTimerHandle))
    (Utilities|Time|ClearandInvalidateTimerbyHandle (Variables|Default|GetTimerHandle)))
  (Class|CombatInterface|SetinShockLoop(Message) (Ability|GetAvatarActorfromActorInfo) false)
  (Variables|/Script/Engine.PlayerController|SetbShowMouseCursor (Variables|Default|GetOwnerPlayerController) true)
  (for _array_element (Variables|Default|GetOutAdditionalTargets)
    (if (.ReturnValue (Utilities|Map|Find (Variables|Default|GetActorToGCParam) _array_element))
      (GameplayCue|RemoveGameplayCueOnActor(Looping) _array_element "(TagName=\"GameplayCue.ShockLoop\")" (.Value (Utilities|Map|Find (Variables|Default|GetActorToGCParam) _array_element)))
      (Ability|HasAuthority
        (:True
          (bind _returnvalue (Class|CombatInterface|IsDead(Message) _array_element))
          (if (not _returnvalue)
            (Class|CombatInterface|SetIsBeingShock(Message) _array_element false)
            (Class|AuraAbilitySystemLibrary|ApplyDamageEffectforDamageEffectParms _array_element (Class|AuraDamageGameplayAbility|GetDamageEffectParamsforTarget _array_element "0, 0, 0")))))))
  (GameplayCue|RemoveGameplayCueOnActor(Looping) (Variables|Default|GetCueTarget) "(TagName=\"GameplayCue.ShockLoop\")" (Variables|Default|GetFirstTargetCueParam))
  (if (Variables|Default|GetIsFirstHitIsEnemy)
    (Ability|HasAuthority
      (:True
        (bind _returnvalue_2 (Class|CombatInterface|IsDead(Message) (Variables|Default|GetCueTarget)))
        (if _returnvalue_2
          _
          (else
            (Class|CombatInterface|SetIsBeingShock(Message) (Variables|Default|GetCueTarget) false)
            (Class|AuraAbilitySystemLibrary|ApplyDamageEffectforDamageEffectParms (Variables|Default|GetCueTarget) (Class|AuraDamageGameplayAbility|GetDamageEffectParamsforTarget (Variables|Default|GetCueTarget) "0, 0, 0")))))
      (:False
        _)))
  (Utilities|Map|Clear (Variables|Default|GetActorToGCParam))
  (Utilities|Array|Clear (Variables|Default|GetOutAdditionalTargets))
  (Variables|Default|SetIsFirstHitIsEnemy false)
  (Variables|Default|SetCueTarget 0)
  (Variables|Default|SetHeldTime 0.0)
  (Ability|CommitAbilityCooldown false))

(fn SpreadBeam
  (for _array_element (Variables|Default|GetOutAdditionalTargets)
    (GameplayCue|AddGameplayCueOnActor(Looping) _array_element "(TagName=\"GameplayCue.ShockLoop\")" (Ability|GameplayCue|MakeGameplayCueParameters :Location (Variables|Default|GetMouseHitLocation) :SourceObject _array_element :TargetAttachComponent (Variables|/Script/Engine.Actor|GetRootComponent (Variables|Default|GetMouseHitActor))))
    (Class|CombatInterface|SetIsBeingShock(Message) _array_element true)
    (Utilities|Map|Add (Variables|Default|GetActorToGCParam) _array_element (Ability|GameplayCue|MakeGameplayCueParameters :Location (Variables|Default|GetMouseHitLocation) :SourceObject _array_element :TargetAttachComponent (Variables|/Script/Engine.Actor|GetRootComponent (Variables|Default|GetMouseHitActor))))))

(fn ApplyDamagetoHitandAdditionalTarget
  (CallFunction|ApplyDamageSingle (Variables|Default|GetMouseHitActor))
  (for _array_element (Variables|Default|GetOutAdditionalTargets)
    (CallFunction|ApplyDamageSingle _array_element)))

(fn ApplyDamageSingle
  (params (Actor :type Actor%20Object%20Reference))
  (bind _returnvalue (Ability|GetAvatarActorfromActorInfo))
  (bind _returnvalue_2 (Ability|GetAbilitySystemComponent _returnvalue))
  (bind _returnvalue_3 (Ability|GameplayEffect|AssignTagSetbyCallerMagnitude (GameplayEffects|MakeOutgoingSpec _returnvalue_2 (Variables|Default|GetDamageEffectClass) (Math|Conversions|ToFloat(Integer) (Ability|GetAbilityLevel)) (GameplayEffects|MakeEffectContext _returnvalue_2)) "(TagName=\"Damage.Lighting\")" (Class|AuraDamageGameplayAbility|GetDamagebyLevel (Ability|GetAbilityLevel))))
  (Ability|HasAuthority
    (:True
      (GameplayEffects|ApplyGameplayEffectSpecToTarget _returnvalue_2 _returnvalue_3 (Ability|GetAbilitySystemComponent Actor)))))

(fn CostandApplyDamage
  (bind _returnvalue (Ability|CommitAbilityCost false))
  (if _returnvalue
    (CallFunction|ApplyDamagetoHitandAdditionalTarget)
    (else
      (CallFunction|PreparetoEndAbility)
      (Ability|EndAbility))))