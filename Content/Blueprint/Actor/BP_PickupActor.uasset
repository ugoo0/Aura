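; BP_PickupActor is a potion-style pickup that animates and plays sound as it spawns and is consumed.
; On BeginPlay it plays a spawn sound, and a Timeline drives its height offset from InitialLocation and its scale.
; A DoOnce plays the ground-hit sound when the float curve dips below a threshold.
; When the Timeline finishes, sinusoidal rotation and movement take over, and Destroyed plays the consume sound.
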(event EventBeginPlay
  (bind _initiallocation (Variables|Default|GetInitialLocation))
  (bind (_x _y _z) (Math|Vector|BreakVector _initiallocation))
  (Audio|PlaySoundatLocation "/Game/Assets/Sounds/Potions/Spawn/sfx_Potion_Spawn.sfx_Potion_Spawn" (Transformation|GetActorLocation) "0, 0, 0" 1.0 1.0 0.0 0 0 0 0)
  (bind (_direction _float _scale) (Timeline|Timeline Play)
    (:Update
      (Transformation|SetActorLocation (Math|Vector|MakeVector _x _y (+ _z (* _float (Variables|Default|GetMaxFloat)))) false false)
      (Transformation|SetActorScale3D (Math|Conversions|ToVector(Float) _scale))
      (if (< _float -0.1)
        (Utilities|FlowControl|DoOnce false
          (:Completed
            (Audio|PlaySoundatLocation "/Game/Assets/Sounds/Potions/HitGround/sfx_Potion_HitGround.sfx_Potion_HitGround" (Transformation|GetActorLocation) "0, 0, 0" 1.0 1.0 0.0 0 0 0 0)))))
    (:Finished
      (Class|AuraEffectActor|StartSinusoidalRotates)
      (Class|AuraEffectActor|StartSinusoidalMovement))))

(event Collision|EventActorBeginOverlap
  (params (OtherActor :type Actor%20Object%20Reference)))

(event EventTick
  (params (DeltaSeconds :type Float%20%28single-precision%29)))

(event EventDestroyed
  (Audio|PlaySoundatLocation "/Game/Assets/Sounds/Potions/Consume/sfx_Potion_Consume.sfx_Potion_Consume" (Transformation|GetActorLocation) "0, 0, 0" 1.0 1.0 0.0 0 0 0 0))

(fn ConstructionScript)