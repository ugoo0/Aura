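; Gameplay Ability for a melee attack, using the avatar's CombatInterface for montages, target and socket locations.
; It picks a random tag-montage pair, faces the combat target, plays the montage and waits for that tag's gameplay event.
; The event gathers live players around the tagged socket within AttackRadius and damages each, calling EndAbility inside the loop.
; The ability also ends when the montage completes, is interrupted or is cancelled.
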(event Ability|EventActivateAbility
  (bind _output_get (Variables|Default|SetAvatarActor (.AvatarActor (Utilities|Struct|BreakGameplayAbilityActorInfo (Ability|GetActorInfo)))))
  (bind _ascombat_interface (Utilities|Casting|CastToCombatInterface _output_get))
  (if (> (Utilities|Array|Length (Class|CombatInterface|GetTagstoMontage _ascombat_interface)) 0)
    (Variables|Default|SetTagToMontage (Utilities|Array|Get(acopy) (Class|CombatInterface|GetTagstoMontage _ascombat_interface) (Math|Random|RandomIntegerinRange 0 (- (Utilities|Array|Length (Class|CombatInterface|GetTagstoMontage _ascombat_interface)) 1))))
    (bind _returnvalue (Class|CombatInterface|GetCombatTarget _ascombat_interface))
    (Class|CombatInterface|FacingtoTarget _ascombat_interface (Transformation|GetActorLocation _returnvalue))
    (|PlayMontageandWaitProxy "None" (.Montage (Utilities|Struct|BreakTagsToMontage (Variables|Default|GetTagToMontage))) 1.0 "None" true 1.0 0.0
      (:then
        (Ability|Tasks|WaitGameplayEvent (.GameplayTag (Utilities|Struct|BreakTagsToMontage (Variables|Default|GetTagToMontage))) 0
          (:EventReceived
            (Development|PrintString "receivedEvent")
            (bind _outoverlayactors (Class|AuraAbilitySystemLibrary|GetLivePlayerswithRadius (Variables|Default|GetAvatarActor) (Utilities|Array|MakeArray (Variables|Default|GetAvatarActor)) (Class|CombatInterface|GetCombatSocketLocation _ascombat_interface (.GameplayTag (Utilities|Struct|BreakTagsToMontage (Variables|Default|GetTagToMontage)))) (Variables|Default|GetAttackRadius)))
            (for _array_element _outoverlayactors
              (Class|AuraDamageGameplayAbility|CauseDamagetoTarget _array_element (Variables|Default|GetTagsGet%20Hurt))
              (Ability|EndAbility)))))
      (:OnCompleted
        (Ability|EndAbility :!label _label))
      (:OnInterrupted
        (goto _label))
      (:OnCancelled
        (goto _label)))
    (else
      (Ability|EndAbility))))

(event Ability|EventOnEndAbility
  (params (bWasCancelled :type Boolean)))