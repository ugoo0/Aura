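; BP_FlamePillar is a flame pillar actor whose fire light varies in intensity to suggest flickering flame.
; On BeginPlay it randomly picks one of two timelines, each driving the FireLight intensity from its curve scaled by BaseIntensity.
; When a timeline finishes, the random choice runs again, giving an endless, irregular light loop without using Tick.
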(event Custom|SetLightIntensity_1
  (bind _intensity (Timeline|Intensity1 PlayFromStart)
    (:Update
      (Rendering|Components|Light|SetIntensity (Variables|Default|GetFireLight) (* _intensity (Variables|Default|GetBaseIntensity))))
    (:Finished
      (CallFunction|ChooseSetLightEvent))))

(event Custom|SetLightIntensity_2
  (bind _intensity (Timeline|Intensity2 PlayFromStart)
    (:Update
      (Rendering|Components|Light|SetIntensity (Variables|Default|GetFireLight) (* _intensity (Variables|Default|GetBaseIntensity))))
    (:Finished
      (CallFunction|ChooseSetLightEvent))))

(event Custom|ChooseSetLightEvent
  (switch int (Math|Random|RandomIntegerinRange 0 1)
    (:Default
      (CallFunction|SetLightIntensity2 :!label _label))
    (:0
      (CallFunction|SetLightIntensity1))
    (:1
      (goto _label))))

(event EventBeginPlay
  (CallFunction|ChooseSetLightEvent))

(event Collision|EventActorBeginOverlap
  (params (OtherActor :type Actor%20Object%20Reference)))

(event EventTick
  (params (DeltaSeconds :type Float%20%28single-precision%29)))

(fn ConstructionScript)