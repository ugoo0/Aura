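; Enemy gameplay ability that summons minions around the avatar's battlefield, using a shaman summon montage and ground VFX at each shuffled spawn location.
; On the montage's attack gameplay event, a delayed loop spawns a random minion class at each location, facing the combat target, with a default controller.
; Each spawn increments the avatar's minion count, and its destruction decrements it.
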(event Custom|OnDestroyed_Event
  (params (DestroyedActor :type Actor%20Object%20Reference))
  (Class|CombatInterface|AddMinionCount(Message) (Ability|GetAvatarActorfromActorInfo) -1))

(event Ability|EventActivateAbility
  (bind _returnvalue (Class|AuraSummonAbility|GetSpawnLocations))
  (bind _output_get (Variables|Default|SetSpawnLocations _returnvalue))
  (Utilities|Array|Shuffle _output_get)
  (for _array_element (Variables|Default|GetSpawnLocations)
    (Niagara|SpawnSystematLocation "/Game/Assets/Effects/Combat/NS_GroundSummon.NS_GroundSummon" _array_element))
  (|PlayMontageandWaitProxy "None" "/Game/Assets/Enemies/Shaman/Animations/AM_Shaman_Summon.AM_Shaman_Summon" 1.0 "None" true 1.0 0.0
    (:then
      (Ability|Tasks|WaitGameplayEvent "(TagName=\"Montage.Attack.1\")" 0
        (:EventReceived
          (if (< (Variables|Default|GetIndex) (Utilities|Array|Length _output_get)) :!label _label
            (bind _returnvalue_2 (Class|CombatInterface|GetCombatTarget(Message) (Ability|GetAvatarActorfromActorInfo)))
            (bind _returnvalue_3 (Class|AuraSummonAbility|GetSpawnClassRandom))
            (bind _returnvalue_4 (Game|SpawnActorfromClass _returnvalue_3 (Math|Transform|MakeTransform (+ (Utilities|Array|Get(acopy) _output_get (Variables|Default|GetIndex)) "0.000000,0.000000,50.000000") (Math|Rotator|FindLookatRotation (+ (Utilities|Array|Get(acopy) _output_get (Variables|Default|GetIndex)) "0.000000,0.000000,50.000000") (Transformation|GetActorLocation _returnvalue_2))) "AlwaysSpawn" "MultiplyWithRoot" 0 0))
            (Pawn|SpawnDefaultController _returnvalue_4)
            (Game|AssignOnDestroyed _returnvalue_4 (delegate Custom|OnDestroyed_Event))
            (Class|CombatInterface|AddMinionCount(Message) (Ability|GetAvatarActorfromActorInfo) 1)
            (Utilities|FlowControl|Delay 0.2)
            (Math|Integer|IncrementInt (Variables|Default|GetIndex)
              (:%20%20
                (goto _label)))))))))

(event Ability|EventOnEndAbility
  (params (bWasCancelled :type Boolean)))