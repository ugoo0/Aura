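; Fireball projectile for the Fire Blast offensive ability that flies out, returns to its owner and explodes.
; On the server, StartTimeLine runs a timeline that moves it forward to an apex point, then a second that pulls it back toward the owner's current location.
; Once within explode distance of the owner, it calls OnHit, broadcasts radial damage to nearby live players other than the owner, and destroys itself.
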(event EventBeginPlay)

(event Collision|EventActorBeginOverlap
  (params (OtherActor :type Actor%20Object%20Reference)))

(event EventTick
  (params (DeltaSeconds :type Float%20%28single-precision%29)))

(event EventStartTimeLine
  (bind _returnvalue (Components|GetOwner))
  (bind _returnvalue_2 (Transformation|GetActorLocation))
  (Networking|SwitchHasAuthority
    (:Authority
      (Variables|Default|SetInitLocation (Transformation|GetActorLocation))
      (Variables|Default|SetInitForward (Transformation|GetActorForwardVector))
      (Variables|Default|SetApexLocation (+ (* (Variables|Default|GetInitForward) (Variables|Default|GetApexDistance)) (Variables|Default|GetInitLocation)))
      (bind _expendfloat (Timeline|ExpendTimeline Play)
        (:Update
          (Transformation|SetActorLocation (Math|Vector|Lerp(Vector) (Variables|Default|GetInitLocation) (Variables|Default|GetApexLocation) _expendfloat) false false))
        (:Finished
          (Variables|Default|SetbOverlay false)
          (bind _backfloat (Timeline|BackTimeline Play)
            (:Update
              (Transformation|SetActorLocation (Math|Vector|Lerp(Vector) (Variables|Default|GetApexLocation) (Transformation|GetActorLocation (Components|GetOwner)) _backfloat) false false)
              (if (< (Math|Vector|VectorLength (- (Transformation|GetActorLocation) (Transformation|GetActorLocation (Components|GetOwner)))) (Variables|Default|GetExplodeDistance))
                (Class|AuraProjectile|OnHit)
                (bind _outoverlayactors (Class|AuraAbilitySystemLibrary|GetLivePlayerswithRadius _returnvalue (Utilities|Array|MakeArray _returnvalue self) _returnvalue_2 (Variables|Default|GetRadialDamageOuterRadius)))
                (Class|AuraFireBall|BroadCastFinalExplodeDelegatetoTargets _outoverlayactors true _returnvalue_2)
                (Actor|DestroyActor)))))))))

(fn ConstructionScript)