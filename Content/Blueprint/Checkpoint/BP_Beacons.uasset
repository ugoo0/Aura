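; BP_Beacons is a checkpoint beacon that glows when reached by an actor implementing AuraPlayerInterface.
; Its sphere overlap, bound at BeginPlay, calls HandleGlowEffect, defined outside these graphs, and sets the Reached flag.
; The CheckpointReached event receives a dynamic material instance and plays the Glow timeline to drive its Glow parameter, scaled by GlowFactor.
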(event Custom|OnComponentBeginOverlap_Event
  (params (OverlappedComponent :type Primitive%20Component%20Object%20Reference) (OtherActor :type Actor%20Object%20Reference) (OtherComp :type Primitive%20Component%20Object%20Reference) (OtherBodyIndex :type Integer) (bFromSweep :type Boolean) (SweepResult :type Hit%20Result%20Structure%20%28by%20ref%29))
  (if (Utilities|DoesObjectImplementInterface OtherActor "/Script/Aura.AuraPlayerInterface")
    (Class|CheckPoint|HandleGlowEffect)
    (Variables|Default|SetbReached true)))

(event EventBeginPlay
  (Collision|AssignOnComponentBeginOverlap (Variables|Default|GetSphere) (delegate Custom|OnComponentBeginOverlap_Event)))

(event EventTick
  (params (DeltaSeconds :type Float%20%28single-precision%29)))

(event EventCheckpointReached
  (params (InstanceDynamic :type Material%20Instance%20Dynamic%20Object%20Reference))
  (bind _glow (Timeline|Glow Play)
    (:Update
      (Rendering|Material|SetScalarParameterValue InstanceDynamic "Glow" (* _glow (Variables|Default|GetGlowFactor)) :!class /Script/Engine.MaterialInstanceDynamic))))

(fn ConstructionScript)