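; BP_EnemyBase is an enemy character Blueprint that handles spawn scaling, dissolve effects and facing a target.
; On BeginPlay a timeline drives the mesh's uniform relative scale.
; Separate mesh and weapon timelines each animate the Dissolve parameter on a dynamic material passed into their events.
; FacingtoTarget feeds a location to Motion Warping as the FacingTarget warp target.
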(event EventBeginPlay
  (bind _scale (Timeline|ScaleTimeline Play)
    (:Update
      (Transformation|SetRelativeScale3D (Variables|Character|GetMesh) (Math|Vector|MakeVector _scale _scale _scale)))))

(event Collision|EventActorBeginOverlap
  (params (OtherActor :type Actor%20Object%20Reference)))

(event EventTick
  (params (DeltaSeconds :type Float%20%28single-precision%29)))

(event EventStartDissolveMeshTimeline
  (params (DynamicMaterial :type Material%20Instance%20Dynamic%20Object%20Reference))
  (bind _newtrack_0 (Timeline|MeshDissolve Play)
    (:Update
      (Rendering|Material|SetScalarParameterValue DynamicMaterial "Dissolve" _newtrack_0 :!class /Script/Engine.MaterialInstanceDynamic))))

(event EventStartDissolveWeaponTimeline
  (params (DynamicMaterial :type Material%20Instance%20Dynamic%20Object%20Reference))
  (bind _newtrack_0 (Timeline|WeaponDissolve Play)
    (:Update
      (Rendering|Material|SetScalarParameterValue DynamicMaterial "Dissolve" _newtrack_0 :!class /Script/Engine.MaterialInstanceDynamic))))

(event EventFacingtoTarget
  (params (TargetLocation :type Vector%20%28by%20ref%29 :default "0, 0, 0"))
  (Class|MotionWarpingComponent|AddorUpdateWarpTargetfromLocation (Variables|Default|GetMotionWarping) "FacingTarget" TargetLocation))

(fn ConstructionScript)