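; Fire bolt actor for the Aura offensive fire ability, with logic for delayed collision and self-cleanup.
; After a brief delay on BeginPlay, it switches its Sphere component to query-only collision.
; Each Tick compares the current location with the previous one and destroys the actor when per-frame travel falls below a fixed distance, making the cutoff frame-rate dependent.
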(event EventBeginPlay
  (Utilities|FlowControl|Delay 0.1)
  (if (Utilities|IsValid (Variables|Default|GetSphere))
    (Collision|SetCollisionEnabled (Variables|Default|GetSphere) "QueryOnly")))

(event Collision|EventActorBeginOverlap
  (params (OtherActor :type Actor%20Object%20Reference)))

(event EventTick
  (params (DeltaSeconds :type Float%20%28single-precision%29))
  (bind _output_get (Variables|Default|SetLastLocation (Variables|Default|GetCurLocation)))
  (bind _output_get_2 (Variables|Default|SetCurLocation (Transformation|GetActorLocation)))
  (if (< (Math|Vector|Distance(Vector) _output_get_2 _output_get) 2e+01)
    (Actor|DestroyActor)))

(fn ConstructionScript)