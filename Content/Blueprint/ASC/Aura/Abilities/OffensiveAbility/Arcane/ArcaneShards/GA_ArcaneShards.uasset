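; Arcane Shards gameplay ability: a mouse-targeted area spell that erupts a series of damaging shards around the chosen point.
; It shows a magic circle until input press, then commits cost and gets level-scaled, capped ground points from a randomly rotated BP_PointCollection.
; A cast montage event commits cooldown and starts a looping timer.
; Each tick fires one shard GameplayCue and applies radial damage, excluding the caster, until cleanup ends the ability.
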(event Custom|SpawnShard
  (bind _returnvalue (Ability|GetAvatarActorfromActorInfo))
  ;[1 1 1] SpawnEffect
  (if (< (Variables|Default|GetCount) (Variables|Default|GetNums))
    (Variables|Default|SetSpawnLocation (Transformation|GetWorldLocation (Utilities|Array|Get(acopy) (Variables|Default|GetGroundPoints) (Variables|Default|GetCount))))
    (Class|GameplayAbility|ExecuteGameplayCuewithParams "(TagName=\"GameplayCue.ArcaneShards\")" (Ability|GameplayCue|MakeGameplayCueParameters :Location (Variables|Default|GetSpawnLocation)))
    (Math|Integer|IncrementInt (Variables|Default|GetCount)
      (:%20%20
        ;[1 0.3281 0.3281] Apply Damage
        (bind _outoverlayactors (Class|AuraAbilitySystemLibrary|GetLivePlayerswithRadius _returnvalue (Utilities|Array|MakeArray _returnvalue) (Variables|Default|GetSpawnLocation) (Variables|Default|GetRadialDamageOuterRadius)))
        (bind _output_get (Variables|Default|SetVictimActors _outoverlayactors))
        (for _array_element _output_get
          (Class|AuraAbilitySystemLibrary|ApplyDamageEffectforDamageEffectParms (Ability|GetAvatarActorfromActorInfo) (Class|AuraDamageGameplayAbility|GetDamageEffectParamsforTarget _array_element (Variables|Default|GetSpawnLocation))))))
    (else
      (Utilities|Time|ClearandInvalidateTimerbyHandle (Variables|Default|GetTimerHandle))
      (Actor|DestroyActor (Variables|Default|GetPointCollectionActor))
      (Variables|Default|SetCount 0)
      (Ability|EndAbility))))

(event Ability|EventActivateAbility
  (Utilities|FlowControl|Sequence
    (:then_0
      (Class|AuraInterface|ShowMagicCircle(Message) (Ability|GetAvatarActorfromActorInfo)))
    (:then_1
      (Ability|Tasks|WaitInputPress false
        (:OnPress
          (Utilities|FlowControl|Sequence
            (:then_0
              (bind _returnvalue (Ability|CommitAbilityCost false))
              (if (not _returnvalue)
                (Ability|EndAbility)))
            (:then_1
              ;[1 1 1] HideMagicCircle
              (Class|AuraInterface|HideMagicCircle(Message) (Ability|GetAvatarActorfromActorInfo))
              ;[1 1 1] CollectInfo
              (bind _datahandle (|TargetDataUnderMouse)
                (:ValidData
                  (Variables|Default|SetMouseHitPoint (.ImpactPoint (Collision|BreakHitResult (Ability|TargetData|GetHitResultfromTargetData _datahandle))))
                  (bind _returnvalue_2 (Game|SpawnActorfromClass "/Game/Blueprint/ASC/Aura/Abilities/OffensiveAbility/Arcane/ArcaneShards/BP_PointCollection.BP_PointCollection_C" (Math|Transform|MakeTransform (.ImpactPoint (Collision|BreakHitResult (Ability|TargetData|GetHitResultfromTargetData _datahandle)))) "AlwaysSpawn" "MultiplyWithRoot" (Ability|GetAvatarActorfromActorInfo) 0))
                  (Variables|Default|SetNumPointsSpawn (Math|Integer|Min(Integer) (Variables|Default|GetMaXNumShards) (Ability|GetAbilityLevel)))
                  (bind _output_get (Variables|Default|SetPointCollectionActor _returnvalue_2))
                  (bind _output_get_2 (Variables|Default|SetGroundPoints (Class|PointCollection|GetGroundPoints _output_get (Variables|Default|GetMouseHitPoint) (Variables|Default|GetNumPointsSpawn) (Math|Random|RandomFloatinRange 0.0 1.8e+02))))
                  (Variables|Default|SetNums (Utilities|Array|Length _output_get_2))
                  (Variables|Default|SetCount 0))))
            (:then_2
              ;[1 1 1] Montage
              (Class|CombatInterface|FacingtoTarget(Message) (Ability|GetAvatarActorfromActorInfo) (Variables|Default|GetMouseHitPoint))
              (|PlayMontageandWaitProxy "None" "/Game/Assets/Characters/Aura/Animations/Abilities/AM_Cast_ArcaneShards.AM_Cast_ArcaneShards" 1.0 "None" false 1.0 0.0
                (:then
                  (Ability|Tasks|WaitGameplayEvent "(TagName=\"Event.Montage.ArcaneShards\")" 0 true
                    (:EventReceived
                      ;[1 1 1] SpawnEffect
                      (Ability|CommitAbilityCooldown false)
                      (bind _returnvalue_3 (Utilities|Time|SetTimerbyEvent (delegate Custom|SpawnShard) (Variables|Default|GetdeltaTimeSpawn) true -0.2))
                      (Variables|Default|SetTimerHandle _returnvalue_3))))))))))))

(event Ability|EventOnEndAbility
  (params (bWasCancelled :type Boolean)))