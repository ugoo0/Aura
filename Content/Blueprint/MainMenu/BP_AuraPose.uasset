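; BP_AuraPose is a main menu scene actor that animates a posed firebolt and decal behind the menu.
; On BeginPlay it plays menu music, creates WBP_MainMenu, and switches the player to UI-only input with the cursor shown.
; Each tick bobs the firebolt around its starting height on a wrapped sine wave and slowly spins the decal around its roll axis.
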(event EventBeginPlay
  (bind _returnvalue (Game|GetPlayerController 0))
  (Variables|Default|SetFireBoltInitialLocation (Transformation|GetWorldLocation (Variables|Default|Getfirebolt)))
  (Audio|PlaySound2D "/Game/Assets/Sounds/Music/Music_MainMenu.Music_MainMenu" 1.0 1.0 0.0 0 0)
  (if (Utilities|IsValid _returnvalue)
    (bind _returnvalue_2 (UserInterface|CreateWidget "/Game/Blueprint/UI/MainMenu/WBP_MainMenu.WBP_MainMenu_C" _returnvalue))
    (UserInterface|Viewport|AddtoViewport _returnvalue_2 0)
    (Input|SetInputModeUIOnly _returnvalue 0 "DoNotLock" false)
    (Variables|/Script/Engine.PlayerController|SetbShowMouseCursor (Game|GetPlayerController 0) true)))

(event Collision|EventActorBeginOverlap
  (params (OtherActor :type Actor%20Object%20Reference)))

(event EventTick
  (params (DeltaSeconds :type Float%20%28single-precision%29))
  (CallFunction|FloatFireBolt DeltaSeconds)
  (CallFunction|RotateDecal (Utilities|Time|GetWorldDeltaSeconds)))

(fn ConstructionScript)

(fn RotateDecal
  (params (A :type Float%20%28double-precision%29))
  (Transformation|SetWorldRotation (Variables|Default|GetDecal) (Math|Rotator|MakeRotator (+ (* A 12.0) (.Roll (Math|Rotator|BreakRotator (Transformation|GetWorldRotation (Variables|Default|GetDecal))))) 0.0 0.0) false false))

(fn FloatFireBolt
  (params (A :type Float%20%28double-precision%29))
  (bind _fireboltinitiallocation (Variables|Default|GetFireBoltInitialLocation))
  (bind (_x _y _z) (Math|Vector|BreakVector _fireboltinitiallocation))
  (bind _output_get (Variables|Default|SetTime (+ A (Variables|Default|GetTime))))
  (if (>= _output_get 6.283185)
    (Variables|Default|SetTime 0.0))
  (Transformation|SetWorldLocation (Variables|Default|Getfirebolt) (Math|Vector|MakeVector _x _y (+ (* (Variables|Default|GetFloatMaxDistance) (Math|Trig|Sin(Radians) (Variables|Default|GetTime))) _z)) false false))