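; Enemy gameplay ability that performs a ranged attack by firing a projectile at the avatar's combat target.
; It picks a random tagged montage through CombatInterface, turns the avatar toward the target and plays the montage.
; The montage's gameplay event spawns the projectile from the tagged socket with a pitch override.
; The ability ends a short delay after that, when the montage finishes or is cut short, or when no montage is available.
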(event Ability|EventActivateAbility
  (bind _ascombat_interface (Utilities|Casting|CastToCombatInterface (Ability|GetAvatarActorfromActorInfo))
    (:then
      (if (> (Utilities|Array|Length (Class|CombatInterface|GetTagstoMontage _ascombat_interface)) 0)
        (bind _output_get (Variables|Default|SetTagToMontage (Utilities|Array|Get(acopy) (Class|CombatInterface|GetTagstoMontage _ascombat_interface) (Math|Random|RandomIntegerinRange 0 (- (Utilities|Array|Length (Class|CombatInterface|GetTagstoMontage _ascombat_interface)) 1)))))
        (bind _returnvalue (Class|CombatInterface|GetCombatTarget _ascombat_interface))
        (Class|CombatInterface|FacingtoTarget _ascombat_interface (Transformation|GetActorLocation _returnvalue))
        (|PlayMontageandWaitProxy "None" (.Montage (Utilities|Struct|BreakTagsToMontage _output_get)) 1.0 "None" true 1.0 0.0
          (:then
            (Ability|Tasks|WaitGameplayEvent (.MontageGameplayTag (Utilities|Struct|BreakTagsToMontage _output_get)) 0 true
              (:EventReceived
                (Class|AuraProjectileSpell|SpawnProjectile (Transformation|GetActorLocation _returnvalue) (.SocketGameplayTag (Utilities|Struct|BreakTagsToMontage _output_get)) true 1e+01)
                (Utilities|FlowControl|Delay 1.0)
                (Ability|EndAbility))))
          (:OnCompleted
            (Ability|EndAbility :!label _label))
          (:OnInterrupted
            (goto _label))
          (:OnCancelled
            (goto _label)))
        (else
          (Ability|EndAbility :!label _label_2))))
    (:CastFailed
      (goto _label_2))))

(event Ability|EventOnEndAbility
  (params (bWasCancelled :type Boolean)))