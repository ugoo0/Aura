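; GA_ListenForEvents is a passive Aura gameplay ability that turns attribute gameplay events into effects on its owner.
; On activation it waits for events under the Attribute tag, including child tags.
; Each event builds a spec from BasedEventEffectClass, setting set-by-caller magnitudes for every listed tag: the event magnitude for the exact match, zero otherwise.
; The spec is then applied to self; a debug string prints on activation.
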(event Ability|EventActivateAbility
  (bind _returnvalue (Ability|GetAbilitySystemComponentfromActorInfo))
  (Development|PrintString "ListenForEveents" true true "(R=1.000000,G=0.131160,B=0.676998,A=1.000000)" 5.0)
  (bind _payload (Ability|Tasks|WaitGameplayEvent "(TagName=\"Attribute\")" 0 false false)
    (:EventReceived
      (Variables|Default|SetEventTag (.EventTag (Utilities|Struct|BreakGameplayEventData _payload)))
      (Variables|Default|SetEventMagnitude (.EventMagnitude (Utilities|Struct|BreakGameplayEventData _payload)))
      (Variables|Default|SetSpec (GameplayEffects|MakeOutgoingSpec _returnvalue (Variables|Default|GetBasedEventEffectClass) 1.0 (GameplayEffects|MakeEffectContext _returnvalue)))
      (for _array_element (Variables|Default|GetGameplayTags)
        (if (GameplayTags|MatchesTag (Variables|Default|GetEventTag) _array_element true)
          (Ability|GameplayEffect|AssignTagSetbyCallerMagnitude (Variables|Default|GetSpec) _array_element (Variables|Default|GetEventMagnitude))
          (else
            (Ability|GameplayEffect|AssignTagSetbyCallerMagnitude (Variables|Default|GetSpec) _array_element 0.0))))
      (GameplayEffects|ApplyGameplayEffectSpecToSelf (Ability|GetAbilitySystemComponentfromActorInfo) (Variables|Default|GetSpec)))))

(event Ability|EventOnEndAbility
  (params (bWasCancelled :type Boolean)))