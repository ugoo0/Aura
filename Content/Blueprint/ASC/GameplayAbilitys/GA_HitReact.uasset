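; GA_HitReact is a gameplay ability that plays the avatar's hit-react animation while a GE_HitReact effect is applied to the owner.
; It gets the montage through CombatInterface and plays it with a wait task.
; On completion it removes the effect by stored handle, then ends after a short delay.
; Interrupted and cancelled paths only print debug text, leaving the effect and ability active.
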(event Ability|EventActivateAbility
  (bind _returnvalue (Ability|ApplyGameplayEffectToOwner "/Game/Blueprint/ASC/GameplayEffect/Damage/GE_HitReact.GE_HitReact_C"))
  (Variables|Default|SetGEHandle _returnvalue)
  (bind _ascombat_interface (Utilities|Casting|CastToCombatInterface (Ability|GetAvatarActorfromActorInfo)))
  (Development|PrintString "11111")
  (bind _returnvalue_2 (Class|CombatInterface|GetHitReactMontage _ascombat_interface))
  (|PlayMontageandWaitProxy "None" _returnvalue_2 1.0 "None" true 1.0 0.0
    (:OnCompleted
      (Ability|RemoveGameplayEffectFromOwnerWithHandle (Variables|Default|GetGEHandle))
      (Utilities|FlowControl|Delay 2.0)
      (Ability|EndAbility)
      (Development|PrintString "222222"))
    (:OnInterrupted
      (Development|PrintString "interrupted"))
    (:OnCancelled
      (Development|PrintString "cancelled"))))

(event Ability|EventOnEndAbility
  (params (bWasCancelled :type Boolean)))