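; GA_FireBlast is the Fire Blast offensive Gameplay Ability that spawns fireballs and deals explosion damage.
; On activation it commits, calls SpawnFireBalls and ends immediately, or just ends if the commit fails.
; OnFinalExplode applies damage only with authority, rebuilding damage effect params for the target from the incoming radial origin, radii, death impulse and knockback force.
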(event Ability|EventActivateAbility
  (bind _returnvalue (Ability|CommitAbility))
  (if _returnvalue
    (Class|AuraFireBlast|SpawnFireBalls)
    (Ability|EndAbility)
    (else
      (Ability|EndAbility))))

(event Ability|EventOnEndAbility
  (params (bWasCancelled :type Boolean)))

(event EventOnFinalExplode
  (params (Target :type Actor%20Object%20Reference) (Params :type Damage%20Effect%20Params%20Structure%20%28by%20ref%29))
  (bind (_worldcontext _damageeffectclass _sourceasc _targetasc _basedamage _damagetype _abilitylevel _debuffchance _debuffdamage _debuffduration _debufffrequency _deathimpulsemagnitude _deathimpulse _knockbackforcemagnitude _knockbackforce _knockbackchance _bisradialdamage _radialdamageinnerradius _radialdamageouterradius _radialdamageorigin) (Utilities|Struct|BreakDamageEffectParams Params))
  ;[1 1 1] ExplodeDamage
  (Ability|HasAuthority
    (:True
      (Class|AuraAbilitySystemLibrary|ApplyDamageEffectforDamageEffectParms (Ability|GetAvatarActorfromActorInfo) (Class|AuraDamageGameplayAbility|GetDamageEffectParamsforTargetOverride Target false _radialdamageorigin _radialdamageouterradius _radialdamageinnerradius _deathimpulse _knockbackforce)))))